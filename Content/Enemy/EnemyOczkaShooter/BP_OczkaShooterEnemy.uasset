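; Oczka shooter enemy: a flipbook-sprite character that fires projectiles at the player and dies from the first damage it takes.
; Pawn sensing latches player detection, after which Tick keeps it yawed toward the player until death and beyond.
; Within range, latent delays pace the throw animation, movement deactivation and BP_OCZKABullet spawn.
; Death runs once, adding player Stress, disabling collision, playing dying and dead flipbooks, and spawning Velo.
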(event OnSeePawn(PawnSensing)
  (params (Pawn :type Pawn%20Object%20Reference))
  (Utilities|Casting|CastToBP_FirstPersonCharacter Pawn)
  (Variables|Default|Setcanseeplayer true))

(event EventTick
  (params (DeltaSeconds :type Float%20%28single-precision%29))
  (bind _paperflipbook (Variables|Default|GetPaperFlipbook))
  (if (Variables|Default|Getcanseeplayer)
    (Transformation|SetActorRotation (Math|Rotator|MakeRotator 0.0 0.0 (.yaw (Math|Rotator|FindLookatRotation (Transformation|GetActorLocation) (Transformation|GetActorLocation (Game|GetPlayerCharacter 0))))))
    (if (not (Variables|Default|Getdead))
      (if (<= (Transformation|GetDistanceTo (Game|GetPlayerCharacter 0)) 2e+03)
        (Utilities|FlowControl|Delay 1.5)
        (Variables|Default|SetisAttacking true)
        (if (not (Variables|Default|Getdead))
          (Sprite|SetFlipbook _paperflipbook "/Game/Enemy/EnemyOczkaShooter/ATTACK_2/OczkaRzut.OczkaRzut")
          (Components|Activation|Deactivate (Variables|Character|GetCharacterMovement))
          (Utilities|FlowControl|Delay (Class|PaperFlipbookComponent|GetFlipbookLength _paperflipbook))
          (Game|SpawnActorfromClass "/Game/Enemy/EnemyOczkaShooter/BP_OCZKABullet.BP_OCZKABullet_C" (Math|Transform|MakeTransform (Transformation|GetActorLocation) "0, 0, 0" "1.000000,1.000000,1.000000") "Undefined" "MultiplyWithRoot" 0 0)
          (Variables|Default|SetisAttacking false)
          (if (not (Variables|Default|Getdead))
            (Sprite|SetFlipbook (Variables|Default|GetPaperFlipbook) "/Game/Enemy/EnemyOczkaShooter/ATTACK_2/OczkaIdle.OczkaIdle")))))))

(event Game|Damage|EventAnyDamage
  (params (Damage :type Float%20%28single-precision%29) (DamageType :type Damage%20Type%20Object%20Reference) (InstigatedBy :type Controller%20Object%20Reference) (DamageCauser :type Actor%20Object%20Reference))
  (bind _paperflipbook (Variables|Default|GetPaperFlipbook))
  (Utilities|FlowControl|DoOnce false
    (:Completed
      (Variables|Default|Setdead true)
      (bind _asbp_first_person_character (Utilities|Casting|CastToBP_FirstPersonCharacter (Game|GetPlayerCharacter 0)))
      (Variables|/Game/FirstPerson/Blueprints/BP_FirstPersonCharacter.BP_FirstPersonCharacter_C|SetStress _asbp_first_person_character (+ (Variables|/Game/FirstPerson/Blueprints/BP_FirstPersonCharacter.BP_FirstPersonCharacter_C|GetStress _asbp_first_person_character) 10))
      (Components|Activation|Deactivate (Variables|Character|GetCharacterMovement))
      (Sprite|SetFlipbook _paperflipbook "/Game/Enemy/EnemyOczkaShooter/DYING/OczkaDying.OczkaDying")
      (Collision|SetActorEnableCollision false)
      (Utilities|FlowControl|Delay (Class|PaperFlipbookComponent|GetFlipbookLength _paperflipbook))
      (Sprite|SetFlipbook (Variables|Default|GetPaperFlipbook) "/Game/Enemy/EnemyOczkaShooter/DYING/oczkaDead.oczkaDead")
      (Game|SpawnActorfromClass "/Game/Blueprints/Velo/Velo.Velo_C" (Math|Transform|MakeTransform (Transformation|GetActorLocation) "0, 0, 0" "1.000000,1.000000,1.000000") "Undefined" "MultiplyWithRoot" 0 0))))

(fn ConstructionScript)