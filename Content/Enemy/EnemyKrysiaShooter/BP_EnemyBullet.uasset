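; Enemy projectile that flies toward the player and raises the first-person character's Stress on contact.
; On BeginPlay it locks its travel direction toward the player's position and starts a timer that destroys it after a fixed lifetime.
; Tick moves it along that straight line without sweep while turning its yaw to face the player.
; Hits are found by polling the Sphere's overlap each frame; a hit adds Stress and destroys the bullet.
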(event Custom|CustomEvent
  (Actor|DestroyActor))

(event EventBeginPlay
  (bind _returnvalue (Transformation|GetActorLocation))
  (bind _returnvalue_2 (Game|GetPlayerCharacter 0))
  (bind _returnvalue_3 (Transformation|GetActorLocation _returnvalue_2))
  (bind _returnvalue_4 (Math|Rotator|FindLookatRotation _returnvalue _returnvalue_3))
  (Variables|Default|SetKierunek (Math|Vector|GetForwardVector (Math|Rotator|MakeRotator (.roll _returnvalue_4) (.pitch _returnvalue_4) (.yaw _returnvalue_4))))
  (Utilities|Time|SetTimerbyEvent (delegate Custom|CustomEvent) 1e+01))

(event EventTick
  (params (DeltaSeconds :type Float%20%28single-precision%29))
  (Transformation|SetActorLocation (+ (Transformation|GetActorLocation) (* (* (Variables|Default|GetKierunek) (Variables|Default|Getspeed)) (Utilities|Time|GetWorldDeltaSeconds))) false false)
  (if true
    (Transformation|SetActorRotation (Math|Rotator|MakeRotator 0.0 0.0 (.yaw (Math|Rotator|FindLookatRotation (Transformation|GetActorLocation) (Transformation|GetActorLocation (Game|GetPlayerCharacter 0))))))
    (bind _asbp_first_person_character (Utilities|Casting|CastToBP_FirstPersonCharacter (Game|GetPlayerCharacter 0)))
    (if (Collision|IsOverlappingActor (Variables|Default|GetSphere) _asbp_first_person_character :!class /Script/Engine.PrimitiveComponent)
      (Variables|/Game/FirstPerson/Blueprints/BP_FirstPersonCharacter.BP_FirstPersonCharacter_C|SetStress _asbp_first_person_character (+ (Variables|/Game/FirstPerson/Blueprints/BP_FirstPersonCharacter.BP_FirstPersonCharacter_C|GetStress _asbp_first_person_character) 15))
      (Actor|DestroyActor))))

(fn ConstructionScript)