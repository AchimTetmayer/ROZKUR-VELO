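; Shooter enemy Blueprint with flipbook animation that fires at the first-person player and dies from the first damage it takes.
; Once PawnSensing spots the player, Tick permanently yaws it toward them and, within range, runs a Delay-paced attack that halts movement, plays the reused melee flipbook and spawns BP_EnemyBullet.
; Death raises the player's Stress, disables movement and collision, shows death and corpse flipbooks, then destroys the actor.
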(event OnSeePawn(PawnSensing)
  (params (Pawn :type Pawn%20Object%20Reference))
  (Utilities|Casting|CastToBP_FirstPersonCharacter Pawn)
  (Variables|Default|Setcanseeplayer true))

(event EventTick
  (params (DeltaSeconds :type Float%20%28single-precision%29))
  (bind _paperflipbook (Variables|Default|GetPaperFlipbook))
  (bind _charactermovement (Variables|Character|GetCharacterMovement))
  (if (Variables|Default|Getcanseeplayer)
    (Transformation|SetActorRotation (Math|Rotator|MakeRotator 0.0 0.0 (.yaw (Math|Rotator|FindLookatRotation (Transformation|GetActorLocation) (Transformation|GetActorLocation (Game|GetPlayerCharacter 0))))))
    (if (not (Variables|Default|Getdead))
      (if (<= (Transformation|GetDistanceTo (Game|GetPlayerCharacter 0)) 2e+03)
        (Utilities|FlowControl|Delay 3.0)
        (Variables|Default|SetisAttacking true)
        (Sprite|SetFlipbook _paperflipbook "/Game/Enemy/MeleeAttack_F1.MeleeAttack_F1")
        (Components|Activation|Deactivate _charactermovement)
        (Utilities|FlowControl|Delay (Class|PaperFlipbookComponent|GetFlipbookLength _paperflipbook))
        (Game|SpawnActorfromClass "/Game/Enemy/EnemyShooter/BP_EnemyBullet.BP_EnemyBullet_C" (Math|Transform|MakeTransform (Transformation|GetActorLocation) "0, 0, 0" "1.000000,1.000000,1.000000") "Undefined" "MultiplyWithRoot" 0 0)
        (Variables|Default|SetisAttacking false)
        (if (not (Variables|Default|Getdead))
          (Components|Activation|SetActive _charactermovement true false)
          (Sprite|SetFlipbook (Variables|Default|GetPaperFlipbook) "/Game/Enemy/MeleeMove.MeleeMove"))))))

(event Game|Damage|EventAnyDamage
  (params (Damage :type Float%20%28single-precision%29) (DamageType :type Damage%20Type%20Object%20Reference) (InstigatedBy :type Controller%20Object%20Reference) (DamageCauser :type Actor%20Object%20Reference))
  (bind _paperflipbook (Variables|Default|GetPaperFlipbook))
  (Utilities|FlowControl|DoOnce false
    (:Completed
      (Variables|Default|Setdead true)
      (bind _asbp_first_person_character (Utilities|Casting|CastToBP_FirstPersonCharacter (Game|GetPlayerCharacter 0)))
      (Variables|/Game/FirstPerson/Blueprints/BP_FirstPersonCharacter.BP_FirstPersonCharacter_C|SetStress _asbp_first_person_character (+ (Variables|/Game/FirstPerson/Blueprints/BP_FirstPersonCharacter.BP_FirstPersonCharacter_C|GetStress _asbp_first_person_character) 10))
      (Components|Activation|Deactivate (Variables|Character|GetCharacterMovement))
      (Sprite|SetFlipbook _paperflipbook "/Game/Enemy/meleedeath1.meleedeath1")
      (Collision|SetActorEnableCollision false)
      (Utilities|FlowControl|Delay (Class|PaperFlipbookComponent|GetFlipbookLength _paperflipbook))
      (Sprite|SetFlipbook (Variables|Default|GetPaperFlipbook) "/Game/Enemy/deadbody_Flipbook.deadbody_Flipbook")
      (Utilities|FlowControl|Delay 4.0)
      (Actor|DestroyActor))))

(fn ConstructionScript)