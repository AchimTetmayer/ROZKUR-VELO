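; Boss enemy with Paper2D flipbook visuals that activates once the first-person character's BossStart flag is set.
; Tick turns it to face the player and, within range, fires two bullet types, paced by chained Delays.
; A DoOnce starts an endless AIMoveTo patrol through four marker actors, spawning a Velo below the boss after each stop.
; Damage shrinks the scaled health bar, then death plays flipbooks and destroys the actor; Dead is never set here.
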(event EventBeginPlay
  (Transformation|SetWorldScale3D (Variables|Default|GetHealthBar) (Math|Vector|MakeVector (* (+ (Variables|Default|GetHealth) 1.0) 0.04) 1.0 1.0)))

(event EventTick
  (params (DeltaSeconds :type Float%20%28single-precision%29))
  (bind _asbp_first_person_character (Utilities|Casting|CastToBP_FirstPersonCharacter (Game|GetPlayerCharacter 0)))
  (if (Variables|/Game/FirstPerson/Blueprints/BP_FirstPersonCharacter.BP_FirstPersonCharacter_C|GetBoss_Start _asbp_first_person_character)
    (if true
      (Transformation|SetActorRotation (Math|Rotator|MakeRotator 0.0 0.0 (.yaw (Math|Rotator|FindLookatRotation (Transformation|GetActorLocation) (Transformation|GetActorLocation (Game|GetPlayerCharacter 0))))))
      (if (not (Variables|Default|Getdead))
        (if (<= (Transformation|GetDistanceTo (Game|GetPlayerCharacter 0)) 1e+04)
          (Variables|Default|SetisAttacking true)
          (Utilities|FlowControl|Delay 0.3)
          (Game|SpawnActorfromClass "/Game/Enemy/Boss/BP_BossBullet.BP_BossBullet_C" (Math|Transform|MakeTransform (Transformation|GetActorLocation) "0, 0, 0" "1.000000,1.000000,1.000000") "Undefined" "MultiplyWithRoot" 0 0)
          (Utilities|FlowControl|Delay 0.2)
          (Game|SpawnActorfromClass "/Game/Enemy/Boss/BP_BossBullet2.BP_BossBullet2_C" (Math|Transform|MakeTransform (Transformation|GetActorLocation) "0, 0, 0" "1.000000,1.000000,1.000000") "Undefined" "MultiplyWithRoot" 0 0)
          (Utilities|FlowControl|DoOnce false
            (:Completed
              (bind _outactors (Actor|GetAllActorsOfClass "/Game/Enemy/Boss/A_Move.A_Move_C"))
              (AI|AIMoveTo self "0, 0, 0" (Utilities|Array|Get(acopy) _outactors) 5.0 false :!label _label
                (:OnSuccess
                  (Utilities|FlowControl|Delay 1.5)
                  (Game|SpawnActorfromClass "/Game/Blueprints/Velo/Velo.Velo_C" (Math|Transform|MakeTransform (- (Transformation|GetActorLocation) "0.000000,0.000000,200.000000") "0, 0, 0" "1.000000,1.000000,1.000000") "Undefined" "MultiplyWithRoot" 0 0)
                  (bind _outactors_2 (Actor|GetAllActorsOfClass "/Game/Enemy/Boss/B_Move.B_Move_C"))
                  (AI|AIMoveTo self "0, 0, 0" (Utilities|Array|Get(acopy) _outactors_2) 5.0 false
                    (:OnSuccess
                      (Utilities|FlowControl|Delay 6.0)
                      (Game|SpawnActorfromClass "/Game/Blueprints/Velo/Velo.Velo_C" (Math|Transform|MakeTransform (- (Transformation|GetActorLocation) "0.000000,0.000000,200.000000") "0, 0, 0" "1.000000,1.000000,1.000000") "Undefined" "MultiplyWithRoot" 0 0)
                      (bind _outactors_3 (Actor|GetAllActorsOfClass "/Game/Enemy/Boss/C_Move.C_Move_C"))
                      (AI|AIMoveTo self "0, 0, 0" (Utilities|Array|Get(acopy) _outactors_3) 5.0 false
                        (:OnSuccess
                          (Utilities|FlowControl|Delay 1.5)
                          (Game|SpawnActorfromClass "/Game/Blueprints/Velo/Velo.Velo_C" (Math|Transform|MakeTransform (- (Transformation|GetActorLocation) "0.000000,0.000000,200.000000") "0, 0, 0" "1.000000,1.000000,1.000000") "Undefined" "MultiplyWithRoot" 0 0)
                          (bind _outactors_4 (Actor|GetAllActorsOfClass "/Game/Enemy/Boss/D_Move.D_Move_C"))
                          (AI|AIMoveTo self "0, 0, 0" (Utilities|Array|Get(acopy) _outactors_4) 5.0 false
                            (:OnSuccess
                              (Utilities|FlowControl|Delay 1.5)
                              (Game|SpawnActorfromClass "/Game/Blueprints/Velo/Velo.Velo_C" (Math|Transform|MakeTransform (- (Transformation|GetActorLocation) "0.000000,0.000000,200.000000") "0, 0, 0" "1.000000,1.000000,1.000000") "Undefined" "MultiplyWithRoot" 0 0)
                              (goto _label))))))))))))))))

(event Game|Damage|EventAnyDamage
  (params (Damage :type Float%20%28single-precision%29) (DamageType :type Damage%20Type%20Object%20Reference) (InstigatedBy :type Controller%20Object%20Reference) (DamageCauser :type Actor%20Object%20Reference))
  (bind _paperflipbook (Variables|Default|GetPaperFlipbook))
  (bind _asbp_first_person_character (Utilities|Casting|CastToBP_FirstPersonCharacter (Game|GetPlayerCharacter 0)))
  (if (Variables|/Game/FirstPerson/Blueprints/BP_FirstPersonCharacter.BP_FirstPersonCharacter_C|GetBoss_Start _asbp_first_person_character)
    (Development|PrintString (Utilities|String|ToString(Float) (Variables|Default|GetHealth)))
    (Variables|Default|SetHealth (- (Variables|Default|GetHealth) Damage))
    (Transformation|SetWorldScale3D (Variables|Default|GetHealthBar) (Math|Vector|MakeVector (* (+ (Variables|Default|GetHealth) 1.0) 0.04) 1.0 1.0))
    (if (< (Variables|Default|GetHealth) 0.0)
      (Components|Activation|Deactivate (Variables|Character|GetCharacterMovement))
      (Sprite|SetFlipbook _paperflipbook "/Game/Enemy/meleedeath1.meleedeath1")
      (Collision|SetActorEnableCollision false)
      (Utilities|FlowControl|Delay (Class|PaperFlipbookComponent|GetFlipbookLength _paperflipbook))
      (Sprite|SetFlipbook (Variables|Default|GetPaperFlipbook) "/Game/Enemy/deadbody_Flipbook.deadbody_Flipbook")
      (Utilities|FlowControl|Delay 4.0)
      (Actor|DestroyActor))))

(fn ConstructionScript)