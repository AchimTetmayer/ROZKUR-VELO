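; Boss projectile that flies at a predicted player position and raises the player's Stress on contact.
; On BeginPlay it fixes its direction using the player's velocity, randomly scaled in X and Y, and starts a lifetime timer.
; Tick moves it straight without sweep, turns its yaw toward the player and polls Sphere overlaps.
; It destroys itself on hitting the player or the first found BP_b_platfrom, or when the timer expires.
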(event Custom|CustomEvent
  (Actor|DestroyActor))

(event EventBeginPlay
  (bind _returnvalue (Math|Random|RandomFloat))
  (bind _returnvalue_2 (Math|Random|RandomFloat))
  (bind _returnvalue_3 (Game|GetPlayerCharacter 0))
  (bind _returnvalue_4 (Game|GetPlayerCharacter 0))
  (bind _returnvalue_5 (Transformation|GetActorLocation))
  (bind _returnvalue_6 (Transformation|GetActorLocation _returnvalue_3))
  (bind _returnvalue_7 (Transformation|GetVelocity _returnvalue_4))
  (bind _returnvalue_8 (+ _returnvalue 1.0))
  (bind _returnvalue_9 (+ _returnvalue_2 1.0))
  (bind _returnvalue_10 (* _returnvalue_7 (Math|Vector|MakeVector _returnvalue_9 _returnvalue_8 1.0)))
  (bind _returnvalue_11 (+ _returnvalue_10 _returnvalue_6))
  (bind _returnvalue_12 (Math|Rotator|FindLookatRotation _returnvalue_5 _returnvalue_11))
  (Variables|Default|SetKierunek (Math|Vector|GetForwardVector (Math|Rotator|MakeRotator (.roll _returnvalue_12) (.pitch _returnvalue_12) (.yaw _returnvalue_12))))
  (Utilities|Time|SetTimerbyEvent (delegate Custom|CustomEvent) 1e+01))

(event EventTick
  (params (DeltaSeconds :type Float%20%28single-precision%29))
  (bind _outactors (Actor|GetAllActorsOfClass "/Game/Enviro/boss/BP_b_platfrom.BP_b_platfrom_C"))
  (if (Collision|IsOverlappingActor (Variables|Default|GetSphere) (Utilities|Array|Get(acopy) _outactors) :!class /Script/Engine.PrimitiveComponent)
    (Actor|DestroyActor)
    (else
      (Transformation|SetActorLocation (+ (Transformation|GetActorLocation) (* (* (Variables|Default|GetKierunek) (Variables|Default|Getspeed)) (Utilities|Time|GetWorldDeltaSeconds))) false false)
      (if true
        (Transformation|SetActorRotation (Math|Rotator|MakeRotator 0.0 0.0 (.yaw (Math|Rotator|FindLookatRotation (Transformation|GetActorLocation) (Transformation|GetActorLocation (Game|GetPlayerCharacter 0))))))
        (bind _asbp_first_person_character (Utilities|Casting|CastToBP_FirstPersonCharacter (Game|GetPlayerCharacter 0)))
        (if (Collision|IsOverlappingActor (Variables|Default|GetSphere) _asbp_first_person_character :!class /Script/Engine.PrimitiveComponent)
          (Variables|/Game/FirstPerson/Blueprints/BP_FirstPersonCharacter.BP_FirstPersonCharacter_C|SetStress _asbp_first_person_character (+ (Variables|/Game/FirstPerson/Blueprints/BP_FirstPersonCharacter.BP_FirstPersonCharacter_C|GetStress _asbp_first_person_character) 10))
          (Actor|DestroyActor))))))

(fn ConstructionScript)