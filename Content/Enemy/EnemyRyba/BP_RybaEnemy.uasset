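; BP_RybaEnemy is a flipbook-animated enemy that chases the first-person player and raises their Stress.
; Pawn sensing starts an AI MoveTo, while Tick yaws it toward the player.
; At close range it halts, plays its attack, adds Stress, then resumes.
; Any damage kills it once, adding Stress, disabling collision, playing death animation and sound, and spawning a Velo.
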(event OnSeePawn(PawnSensing)
  (params (Pawn :type Pawn%20Object%20Reference))
  (bind _asbp_first_person_character (Utilities|Casting|CastToBP_FirstPersonCharacter Pawn))
  (Variables|Default|Setcanseeplayer true)
  (if (not (Variables|Default|GetisAttacking))
    (if (not (Variables|Default|Getdead))
      (AI|AIMoveTo self "0, 0, 0" _asbp_first_person_character 5.0 false))))

(event EventTick
  (params (DeltaSeconds :type Float%20%28single-precision%29))
  (bind _paperflipbook (Variables|Default|GetPaperFlipbook))
  (bind _charactermovement (Variables|Character|GetCharacterMovement))
  (if (Variables|Default|Getcanseeplayer)
    (Transformation|SetActorRotation (Math|Rotator|MakeRotator 0.0 0.0 (.yaw (Math|Rotator|FindLookatRotation (Transformation|GetActorLocation) (Transformation|GetActorLocation (Game|GetPlayerCharacter 0))))))
    (if (not (Variables|Default|Getdead))
      (if (<= (Transformation|GetDistanceTo (Game|GetPlayerCharacter 0)) 1e+02)
        (Variables|Default|SetisAttacking true)
        (Sprite|SetFlipbook _paperflipbook "/Game/Enemy/EnemyRyba/MICHU_ATTACK.MICHU_ATTACK")
        (Components|Activation|Deactivate _charactermovement)
        (Utilities|FlowControl|Delay (Class|PaperFlipbookComponent|GetFlipbookLength _paperflipbook))
        (bind _asbp_first_person_character (Utilities|Casting|CastToBP_FirstPersonCharacter (Game|GetPlayerCharacter 0)))
        (Variables|/Game/FirstPerson/Blueprints/BP_FirstPersonCharacter.BP_FirstPersonCharacter_C|SetStress _asbp_first_person_character (+ (Variables|/Game/FirstPerson/Blueprints/BP_FirstPersonCharacter.BP_FirstPersonCharacter_C|GetStress _asbp_first_person_character) 10))
        (Variables|Default|SetisAttacking false)
        (if (not (Variables|Default|Getdead))
          (Components|Activation|SetActive _charactermovement true false)
          (Sprite|SetFlipbook (Variables|Default|GetPaperFlipbook) "/Game/Enemy/EnemyRyba/MICHU_SWIM.MICHU_SWIM")
          (bind _asbp_first_person_character_2 (Utilities|Casting|CastToBP_FirstPersonCharacter (stale OnSeePawn(PawnSensing) Pawn)))
          (Variables|Default|Setcanseeplayer true)
          (if (not (Variables|Default|GetisAttacking))
            (if (not (Variables|Default|Getdead))
              (AI|AIMoveTo self "0, 0, 0" _asbp_first_person_character_2 5.0 false))))))))

(event Game|Damage|EventAnyDamage
  (params (Damage :type Float%20%28single-precision%29) (DamageType :type Damage%20Type%20Object%20Reference) (InstigatedBy :type Controller%20Object%20Reference) (DamageCauser :type Actor%20Object%20Reference))
  (bind _paperflipbook (Variables|Default|GetPaperFlipbook))
  (Utilities|FlowControl|DoOnce false
    (:Completed
      (Variables|Default|Setdead true)
      (Utilities|FlowControl|Sequence
        (:then_0
          (bind _asbp_first_person_character (Utilities|Casting|CastToBP_FirstPersonCharacter (Game|GetPlayerCharacter 0)))
          (Variables|/Game/FirstPerson/Blueprints/BP_FirstPersonCharacter.BP_FirstPersonCharacter_C|SetStress _asbp_first_person_character (+ (Variables|/Game/FirstPerson/Blueprints/BP_FirstPersonCharacter.BP_FirstPersonCharacter_C|GetStress _asbp_first_person_character) 5))
          (Components|Activation|Deactivate (Variables|Character|GetCharacterMovement))
          (Sprite|SetFlipbook _paperflipbook "/Game/Enemy/EnemyRyba/MICHU_DYING.MICHU_DYING")
          (Collision|SetActorEnableCollision false)
          (Utilities|FlowControl|Delay (Class|PaperFlipbookComponent|GetFlipbookLength _paperflipbook))
          (Sprite|SetFlipbook (Variables|Default|GetPaperFlipbook) "/Game/Enemy/EnemyRyba/MICHU_DEAD.MICHU_DEAD")
          (Game|SpawnActorfromClass "/Game/Blueprints/Velo/Velo.Velo_C" (Math|Transform|MakeTransform (Transformation|GetActorLocation) "0, 0, 0" "1.000000,1.000000,1.000000") "Undefined" "MultiplyWithRoot" 0 0))
        (:then_1
          (Audio|PlaySoundatLocation "/Game/FirstPerson/Blueprints/User_Interface__Beep__Button_Click__Plop__Short_SND113031.User_Interface__Beep__Button_Click__Plop__Short_SND113031" (Transformation|GetActorLocation) "0, 0, 0" 1.0 1.0 0.0 "/Game/FirstPerson/Blueprints/Enemy_DeathSoundLocalization.Enemy_DeathSoundLocalization" "/Game/FirstPerson/Blueprints/Velo_SoundLimit.Velo_SoundLimit" 0 0))))))

(fn ConstructionScript)