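; BP_Pistol is a pistol weapon that fires one shot at a time, animated with a Paper2D flipbook.
; ShootWeapon passes through a DoOnce gate, calls FireWeapon and switches the flipbook to the fire animation.
; After a delay equal to that flipbook's length, it restores the idle flipbook and calls ResetWeapon to reopen the gate, so the animation length sets the fire rate.
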(event Custom|ResetWeapon
  (bind _weaponflipbook (Variables|Default|GetWeaponFlipbook))
  (Utilities|FlowControl|DoOnce false) ; enters at Reset
)

(event EventBeginPlay
  (|CallParentFunction) ; Ten węzeł jest wyłączony i nie będzie wywoływany.\nPrzeciągnij gniazda, aby utworzyć funkcjonalność.
)

(event Collision|EventActorBeginOverlap
  (params (OtherActor :type Actor%20Object%20Reference))
  (|CallParentFunction OtherActor) ; Ten węzeł jest wyłączony i nie będzie wywoływany.\nPrzeciągnij gniazda, aby utworzyć funkcjonalność.
)

(event EventTick
  (params (DeltaSeconds :type Float%20%28single-precision%29))
  (|CallParentFunction DeltaSeconds) ; Ten węzeł jest wyłączony i nie będzie wywoływany.\nPrzeciągnij gniazda, aby utworzyć funkcjonalność.
)

(event EventShootWeapon
  (bind _weaponflipbook (Variables|Default|GetWeaponFlipbook))
  (Utilities|FlowControl|DoOnce false
    (:Completed
      (CallFunction|FireWeapon)
      (Sprite|SetFlipbook _weaponflipbook "/Game/Sprites/Weapons/Pistol/PistolFire.PistolFire")
      (Utilities|FlowControl|Delay (Class|PaperFlipbookComponent|GetFlipbookLength _weaponflipbook))
      (Sprite|SetFlipbook (Variables|Default|GetWeaponFlipbook) "/Game/Sprites/Weapons/Pistol/PistolIdle.PistolIdle")
      (CallFunction|ResetWeapon))))

(fn ConstructionScript
  (|CallParentFunction))