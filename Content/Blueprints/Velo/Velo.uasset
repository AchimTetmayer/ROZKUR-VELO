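; Velo is a pickup actor that the player consumes on touch to lower the first-person character's Stress.
; On Tick it turns its yaw toward the player and polls for overlap with that character instead of using an overlap event.
; On contact it subtracts a fixed amount of Stress, sets the character's EatingVelo flag, plays a 2D sound and destroys itself.
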(event EventBeginPlay)

(event Collision|EventActorBeginOverlap
  (params (OtherActor :type Actor%20Object%20Reference)))

(event EventTick
  (params (DeltaSeconds :type Float%20%28single-precision%29))
  (Transformation|SetActorRotation (Math|Rotator|MakeRotator 0.0 0.0 (.yaw (Math|Rotator|FindLookatRotation (Transformation|GetActorLocation) (Transformation|GetActorLocation (Game|GetPlayerCharacter 0))))))
  (bind _asbp_first_person_character (Utilities|Casting|CastToBP_FirstPersonCharacter (Game|GetPlayerCharacter 0)))
  (if (Collision|IsOverlappingActor _asbp_first_person_character :!class /Script/Engine.Actor)
    (Variables|/Game/FirstPerson/Blueprints/BP_FirstPersonCharacter.BP_FirstPersonCharacter_C|SetStress _asbp_first_person_character (- (Variables|/Game/FirstPerson/Blueprints/BP_FirstPersonCharacter.BP_FirstPersonCharacter_C|GetStress _asbp_first_person_character) 15))
    (Variables|/Game/FirstPerson/Blueprints/BP_FirstPersonCharacter.BP_FirstPersonCharacter_C|SetEatingVelo _asbp_first_person_character true)
    (Audio|PlaySound2D "/Game/FirstPerson/Blueprints/Velo.Velo" 1.0 1.0 0.0 0 0)
    (Actor|DestroyActor)))

(fn ConstructionScript)