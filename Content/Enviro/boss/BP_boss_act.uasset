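; Boss-area trigger actor that switches the lighting to alarm lights and lowers a platform when the first-person character enters its Box.
; BeginPlay records the positions of six child actors used as placement markers, then destroys them.
; On overlap it destroys the point lights, spawns Alarm_light actors at the saved positions, and plays a Timeline that lerps the platform from its current height toward 8000 units below.
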(event OnComponentBeginOverlap(Box)
  (params (OverlappedComponent :type Primitive%20Component%20Object%20Reference) (OtherActor :type Actor%20Object%20Reference) (OtherComp :type Primitive%20Component%20Object%20Reference) (OtherBodyIndex :type Integer) (bFromSweep :type Boolean) (SweepResult :type Hit%20Result%20Structure%20%28by%20ref%29))
  (bind _platform (Variables|Default|Getplatform))
  (bind _returnvalue (Transformation|GetWorldLocation _platform))
  (Utilities|Casting|CastToBP_FirstPersonCharacter OtherActor)
  (Components|DestroyComponent (Variables|Default|GetPointLight))
  (Game|SpawnActorfromClass "/Game/Enviro/boss/alarm_light.alarm_light_C" (Math|Transform|MakeTransform (stale EventBeginPlay _output_get) "0.000000,90.000000,0.000000" "1.000000,1.000000,1.000000") "Undefined" "MultiplyWithRoot" 0 0)
  (Game|SpawnActorfromClass "/Game/Enviro/boss/alarm_light.alarm_light_C" (Math|Transform|MakeTransform (stale EventBeginPlay _output_get_2) "0, 0, 0" "1.000000,1.000000,1.000000") "Undefined" "MultiplyWithRoot" 0 0)
  (Game|SpawnActorfromClass "/Game/Enviro/boss/alarm_light.alarm_light_C" (Math|Transform|MakeTransform (stale EventBeginPlay _output_get_3) "0, 0, 0" "1.000000,1.000000,1.000000") "Undefined" "MultiplyWithRoot" 0 0)
  (Game|SpawnActorfromClass "/Game/Enviro/boss/alarm_light.alarm_light_C" (Math|Transform|MakeTransform (stale EventBeginPlay _output_get_4) "0.000000,90.000000,0.000000" "1.000000,1.000000,1.000000") "Undefined" "MultiplyWithRoot" 0 0)
  (Game|SpawnActorfromClass "/Game/Enviro/boss/alarm_light.alarm_light_C" (Math|Transform|MakeTransform (stale EventBeginPlay _output_get_5) "0, 0, 0" "1.000000,1.000000,1.000000") "Undefined" "MultiplyWithRoot" 0 0)
  (Game|SpawnActorfromClass "/Game/Enviro/boss/alarm_light.alarm_light_C" (Math|Transform|MakeTransform (stale EventBeginPlay _output_get_6) "0.000000,90.000000,0.000000" "1.000000,1.000000,1.000000") "Undefined" "MultiplyWithRoot" 0 0)
  (bind _output_get (Variables|Default|Setlocation (.z _returnvalue)))
  (bind _newtrack_0 (Timeline|Timeline Play)
    (:Update
      (Transformation|SetWorldLocation _platform (Math|Vector|MakeVector (.x _returnvalue) (.y _returnvalue) (Math|Float|Lerp (.z _returnvalue) (+ _output_get -8e+03) _newtrack_0)) false false))))

(event EventBeginPlay
  (bind _childactor (Variables|Default|GetChildActor))
  (bind _output_get (Variables|Default|Setpos (Transformation|GetWorldLocation _childactor)))
  (bind _output_get_2 (Variables|Default|Setpos1 (Transformation|GetWorldLocation (Variables|Default|GetChildActor1))))
  (bind _output_get_3 (Variables|Default|Setpos2 (Transformation|GetWorldLocation (Variables|Default|GetChildActor2))))
  (bind _output_get_4 (Variables|Default|Setpos3 (Transformation|GetWorldLocation (Variables|Default|GetChildActor3))))
  (bind _output_get_5 (Variables|Default|Setpos4 (Transformation|GetWorldLocation (Variables|Default|GetChildActor4))))
  (bind _output_get_6 (Variables|Default|Setpos5 (Transformation|GetWorldLocation (Variables|Default|GetChildActor5))))
  (Components|DestroyComponent _childactor))

(fn ConstructionScript)